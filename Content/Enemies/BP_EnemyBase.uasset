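; BP_EnemyBase is a sword-wielding enemy character base with health, melee attack and movement speed presets.
; Damage and percentage healing adjust clamped health, with zero setting a death flag.
; Equipping spawns and attaches a sword then plays the unsheath montage, while unequipping only plays the sheath montage and clears the wielding flag.
; Montage completion or interruption fires dispatchers, and getters expose health, patrol route and combat ranges.
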(event `self.ReceiveAnyDamage`
  (params (Damage :type "Float (single-precision)") (DamageType :type "DamageType Object Reference") (InstigatedBy :type "Controller Object Reference") (DamageCauser :type "Actor Object Reference"))
  (bind _output_get (set `self.Health` (`KismetMathLibrary.FClamp` (- (`self.Health`) Damage) 0.0 (`self.MaxHealth`))))
  (if (<= _output_get 0.0)
    (set `self.IsDead` true)))

(event `/Game/Enemies/AI/BPI_EnemyAI.Attack`
  (`|PlayMontage` (`self.Mesh`) "/Game/RadiantDark/AM_Slash.AM_Slash"
    (:`OnCompleted`
      _)
    (:`OnInterrupted`
      _))
  (`self.OnAttackEnd`))

(event `/Game/Enemies/AI/BPI_EnemyAI.EquipWeapon`
  (bind _returnvalue (`|SpawnActorFromClass` "/Game/Weapons/BP_Sword.BP_Sword_C" (`self.GetTransform`) "Undefined" "MultiplyWithRoot" null null :!label _label))
  (set `self.WeaponActor` _returnvalue)
  (`self.K2_AttachToComponent` _returnvalue (`self.Mesh`) "hand_r_sowrd_Socket" "SnapToTarget" "SnapToTarget" "SnapToTarget" true)
  (set `self.IsWieldingWeapon` true)
  (`self.UnsheathSword`))

(event `Wield Sword`
  (goto _label))

(event `/Game/Enemies/AI/BPI_EnemyAI.UnequipWeapon`
  (`|PlayMontage` (`self.Mesh`) "/Game/RadiantDark/AM_Sheath_Sword.AM_Sheath_Sword" :!label _label_2
    (:`then`
      (set `self.IsWieldingWeapon` false))
    (:`OnCompleted`
      (`self.OnSheathed` :!label _label_3))
    (:`OnInterrupted`
      (goto _label_3))))

(event `SheathSword`
  (goto _label_2))

(event `UnsheathSword`
  (`|PlayMontage` (`self.Mesh`) "/Game/RadiantDark/AM_Unsheath_Sword.AM_Unsheath_Sword"
    (:`OnCompleted`
      _)
    (:`OnInterrupted`
      _))
  (`self.OnUnsheathed`))

(event `/Game/Enemies/AI/BPI_EnemyAI.Heal`
  (params (HealPercent :type "Float (double-precision)"))
  (set `self.Health` (`KismetMathLibrary.FClamp` (+ (`self.Health`) (* HealPercent (`self.MaxHealth`))) 0.0 (`self.MaxHealth`))))

(fn `GetCurrentHealth`
  (returns (Health :type "Float (double-precision)"))
  (return (`self.Health`)))

(fn `GetIdealRange`
  (returns (AttackRadius :type "Float (double-precision)") (DefenseRadius :type "Float (double-precision)"))
  (return 150.0 350.0))

(fn `GetMaxHealth`
  (returns (MaxHealth :type "Float (double-precision)"))
  (return (`self.MaxHealth`)))

(fn `GetPatrolRoute`
  (returns (PatrolRoute :type "/Game/Enemies/AI/BP_PatrolRoute Object Reference"))
  (return (`self.PatrolRoute`)))

(fn `SetMovementSpeed`
  (params (Speed :type "/Game/Enemies/AI/Enums/E_MovementSpeed Enum" :default "NewEnumerator2"))
  (returns (Value :type "Float (double-precision)"))
  (bind _output_get (set `CharacterMovementComponent.MaxWalkSpeed` (select `/Game/Enemies/AI/Enums/E_MovementSpeed` Speed :`NewEnumerator0` 100.0 :`NewEnumerator1` 300.0 :`NewEnumerator3` 500.0 :!type "Float (single-precision)") (`self.CharacterMovement`)))
  (return _output_get))

(fn `UserConstructionScript`)